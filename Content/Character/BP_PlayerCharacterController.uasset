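; BP_PlayerCharacterController is the player controller that owns the player's HUD widget and controls when it is shown and focused.
; On BeginPlay it creates a BP_HUD widget, adds it to the viewport and hides it.
; The StartMenu input calls ActivateFocus on the HUD without changing its visibility.
; ActivateGameOverHud makes the same widget visible and focuses it for game over.
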(event EventBeginPlay
  (bind _returnvalue (UserInterface|CreateWidget "/Game/Character/BP_HUD.BP_HUD_C"))
  (bind _output_get (Variables|Default|SetplayerHud _returnvalue))
  (UserInterface|Viewport|AddtoViewport _output_get 0)
  (Widget|SetVisibility _output_get "Hidden"))

(event Input|ActionEvents|InputActionStartMenu
  (params (Key :type Key%20Structure))
  (bind _playerhud (Variables|Default|GetplayerHud))
  (:Pressed
    (Utilities|IsValid _playerhud
      (:Is%20Valid
        (Default|ActivateFocus _playerhud)))))

(fn ConstructionScript)

(fn ActivateGameOverHud
  (bind _playerhud (Variables|Default|GetplayerHud))
  (Widget|SetVisibility _playerhud "Visible")
  (Default|ActivateFocus _playerhud))