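; Player character Blueprint that links movement state changes to animation and reacts to reaching finish platforms.
; On BeginPlay it caches its AB_PlayerCharacter anim instance, then forwards MovementComponent idle, run, jump, fall, slide and wall-slide events to that instance's matching transition calls.
; PlatformDetector overlaps with actors tagged "Finish" call ActivateFocus on the player controller's HUD.
; Leftover debug prints are disconnected.
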(event OnIdle(MovementComponent)
  (bind _animationinstance (Variables|Default|GetAnimationInstance))
  (Utilities|IsValid _animationinstance
    (:Is%20Valid
      (Default|TransitiontoIdle _animationinstance))))

(event OnSlide(MovementComponent)
  (bind _animationinstance (Variables|Default|GetAnimationInstance))
  (Utilities|IsValid _animationinstance
    (:Is%20Valid
      (Default|TransitiontoSlide _animationinstance))))

(event OnWallSlide(MovementComponent)
  (bind _animationinstance (Variables|Default|GetAnimationInstance))
  (Utilities|IsValid _animationinstance
    (:Is%20Valid
      (Default|TransitiontoWallSlide _animationinstance))))

(event OnComponentBeginOverlap(PlatformDetector)
  (params (OverlappedComponent :type Primitive%20Component%20Object%20Reference) (OtherActor :type Actor%20Object%20Reference) (OtherComp :type Primitive%20Component%20Object%20Reference) (OtherBodyIndex :type Integer) (bFromSweep :type Boolean) (SweepResult :type Hit%20Result%20Structure%20%28by%20ref%29))
  (if (Actor|ActorHasTag OtherActor "Finish")
    (bind _asbp_player_character_controller (Utilities|Casting|CastToBP_PlayerCharacterController (Pawn|GetController)))
    (Default|ActivateFocus (Variables|/Game/Character/BP_PlayerCharacterController.BP_PlayerCharacterController_C|GetplayerHud _asbp_player_character_controller))))

(event OnRun(MovementComponent)
  (bind _animationinstance (Variables|Default|GetAnimationInstance))
  (Utilities|IsValid _animationinstance
    (:Is%20Valid
      (Default|TransitiontoRun _animationinstance))))

(event OnJump(MovementComponent)
  (bind _animationinstance (Variables|Default|GetAnimationInstance))
  (Utilities|IsValid _animationinstance
    (:Is%20Valid
      (Default|TransitiontoJump _animationinstance))))

(event OnFall(MovementComponent)
  (bind _animationinstance (Variables|Default|GetAnimationInstance))
  (Utilities|IsValid _animationinstance
    (:Is%20Valid
      (Default|TransitiontoFall _animationinstance))))

(event EventBeginPlay
  (bind _asab_player_character (Utilities|Casting|CastToAB_PlayerCharacter (Components|SkeletalMesh|GetAnimInstance (Variables|Default|GetSkeletalMeshComponent))))
  (Variables|Default|SetAnimationInstance _asab_player_character))

(fn ConstructionScript)