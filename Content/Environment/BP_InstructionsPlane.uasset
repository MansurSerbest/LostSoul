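; Instructions plane actor that animates a disintegrate material effect on proximity and gently bobs in the air.
; Begin and end overlaps on Box toggle On, with no check on the overlapping actor.
; Tick steps Disintegrate from its starting 1 toward 0 while On, otherwise back, by a frame-rate-dependent amount, feeding the Plane material's Amount parameter.
; Tick also adds a delta-scaled sine of game time to the Plane's height.
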(event OnComponentBeginOverlap(Box)
  (params (OverlappedComponent :type Primitive%20Component%20Object%20Reference) (OtherActor :type Actor%20Object%20Reference) (OtherComp :type Primitive%20Component%20Object%20Reference) (OtherBodyIndex :type Integer) (bFromSweep :type Boolean) (SweepResult :type Hit%20Result%20Structure%20%28by%20ref%29))
  (Variables|Default|SetOn true))

(event OnComponentEndOverlap(Box)
  (params (OverlappedComponent :type Primitive%20Component%20Object%20Reference) (OtherActor :type Actor%20Object%20Reference) (OtherComp :type Primitive%20Component%20Object%20Reference) (OtherBodyIndex :type Integer))
  (Variables|Default|SetOn false))

(event EventTick
  (params (DeltaSeconds :type Float%20%28single-precision%29))
  (bind _plane (Variables|Default|GetPlane))
  (bind _disintegratespeed (Variables|Default|GetDisintegrateSpeed))
  (bind _returnvalue (Transformation|GetWorldLocation _plane))
  (Utilities|FlowControl|Sequence
    (:then_0
      (if (Variables|Default|GetOn)
        (Variables|Default|SetDisintegrate (Math|Float|Clamp(Float) (- (Variables|Default|GetDisintegrate) _disintegratespeed)))
        (else
          (Variables|Default|SetDisintegrate (Math|Float|Clamp(Float) (+ (Variables|Default|GetDisintegrate) _disintegratespeed))))))
    (:then_1
      (Rendering|Material|SetScalarParameterValueonMaterials _plane "Amount" (Variables|Default|GetDisintegrate)))
    (:then_2
      (Transformation|SetWorldLocation _plane (Math|Vector|MakeVector (.x _returnvalue) (.y _returnvalue) (+ (* DeltaSeconds (* (* (Math|Trig|Sin(Radians) (Utilities|Time|GetTimeSeconds)) 0.5) 1e+01)) (.z _returnvalue))) false false))))

(event EventBeginPlay
  (Variables|Default|SetDisintegrate 1.0))

(fn ConstructionScript)