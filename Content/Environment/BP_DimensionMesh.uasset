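; BP_DimensionMesh is an environment mesh with normal and soul dimension variants that can optionally float as a moving platform.
; Tick bobs the active dimension's mesh on a sine wave, using a swept move to detect the player character.
; A detected player moves with the mesh and is flagged as on a moving platform.
; The movement component's jump and fall delegates clear that flag and release the player.
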(event Custom|OnJump
  ;[1 1 1] Bind OnFall and OnJump events to the OnFall and OnJump Delegates of PlayerCharacter
  (Variables|Default|Setm_PlayerCharacter 0)
  (Class|PlayerCharacterMovementComponent|SetIsonMovingPlatform (Actor|GetComponentbyClass (stale EventBeginPlay _asbp_player_character) "/Script/GameProject.PlayerCharacterMovementComponent") false))

(event Custom|OnFall
  ;[1 1 1] Bind OnFall and OnJump events to the OnFall and OnJump Delegates of PlayerCharacter
  (Variables|Default|Setm_PlayerCharacter 0)
  (Class|PlayerCharacterMovementComponent|SetIsonMovingPlatform (Actor|GetComponentbyClass (stale EventBeginPlay _asbp_player_character) "/Script/GameProject.PlayerCharacterMovementComponent") false))

(event EventTick
  (params (DeltaSeconds :type Float%20%28single-precision%29))
  (bind _returnvalue (Utilities|Time|GetTimeSeconds))
  (bind _flloatamplitude (Variables|Default|GetflloatAmplitude))
  (bind _floatspeed (Variables|Default|GetfloatSpeed))
  (bind _returnvalue_2 (* _returnvalue _floatspeed))
  (bind _returnvalue_3 (Math|Trig|Sin(Radians) _returnvalue_2))
  (bind _returnvalue_4 (* _returnvalue_3 _flloatamplitude))
  (if (Variables|Default|Getm_IsFloating)
    ;[1 1 1] Float Mesh until playercharacter is detected
    (if (not (Utilities|IsValid (Variables|Default|Getm_PlayerCharacter)))
      (bind _sweephitresult (Transformation|AddWorldOffset (select (Variables|Default|GetIsNormalDimension) (Variables|Default|GetNormalDimensionMeshComponent) (Variables|Default|GetSoulDimensionMeshComponent)) (Math|Vector|MakeVector 0.0 0.0 (* (Math|Trig|Sin(Radians) (* (Utilities|Time|GetTimeSeconds) (Variables|Default|GetfloatSpeed))) (Variables|Default|GetflloatAmplitude))) true false))
      (if (.bBlockingHit (Collision|BreakHitResult _sweephitresult))
        (bind _asbp_player_character (Utilities|Casting|CastToBP_PlayerCharacter (.HitActor (Collision|BreakHitResult _sweephitresult))))
        (bind _output_get (Variables|Default|Setm_PlayerCharacter _asbp_player_character))
        (Class|PlayerCharacterMovementComponent|SetIsonMovingPlatform (Actor|GetComponentbyClass _output_get "/Script/GameProject.PlayerCharacterMovementComponent") true))
      (else
        ;[1 1 1] Float Playercharacter together with the mesh
        (Transformation|AddActorWorldOffset (Variables|Default|Getm_PlayerCharacter) (Math|Vector|MakeVector 0.0 0.0 _returnvalue_4))
        (Transformation|AddWorldOffset (select (Variables|Default|GetIsNormalDimension) (Variables|Default|GetNormalDimensionMeshComponent) (Variables|Default|GetSoulDimensionMeshComponent)) (Math|Vector|MakeVector 0.0 0.0 _returnvalue_4) false false)
        (Development|PrintString "platfooorom")))))

(event EventBeginPlay
  ;[1 1 1] Bind OnFall and OnJump events to the OnFall and OnJump Delegates of PlayerCharacter
  (bind _asbp_player_character (Utilities|Casting|CastToBP_PlayerCharacter (Pawn|GetControlledPawn (Game|GetPlayerController 0))))
  (Utilities|IsValid (Actor|GetComponentbyClass _asbp_player_character "/Script/GameProject.PlayerCharacterMovementComponent")
    (:Is%20Valid
      (EventDispatchers|BindEventtoOnJump (Actor|GetComponentbyClass _asbp_player_character "/Script/GameProject.PlayerCharacterMovementComponent") (delegate Custom|OnJump))
      (EventDispatchers|BindEventtoOnFall (Actor|GetComponentbyClass _asbp_player_character "/Script/GameProject.PlayerCharacterMovementComponent") (delegate Custom|OnFall)))))

(event EventSwitchtoSoulDimension
  (|CallParentFunction)
  (Variables|Default|SetIsNormalDimension false))

(event EventSwitchtoNormalDimension
  (|CallParentFunction)
  (Variables|Default|SetIsNormalDimension true))

(fn ConstructionScript)